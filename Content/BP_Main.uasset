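; BP_Main builds a 9x9 Paper2D tile board and lets the player click two tiles to swap them.
; BeginPlay fills the board with random tile sets, while RandomBranch counts boom and stone picks to narrow the random range, though it rolls separately from the placed tile.
; Clicks map viewport position to 128-pixel cells, highlight the first selection on a second layer, then swap, or deselect if the tile set matches.
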(event `self.ReceiveBeginPlay`
  (bind _papertilemap (`self.PaperTileMap`))
  (bind _papertilemap_2 (`self.PaperTileMap`))
  (bind _returnvalue (`KismetMathLibrary.RandomIntegerInRange` (`self.Min`) (`self.Max`)))
  (`self.EnableInput` (`GameplayStatics.GetPlayerController` 0))
  (`PaperTileMapComponent.CreateNewTileMap` _papertilemap 9 9 32 32 1.0 true)
  (`PaperTileMapComponent.MakeTileMapEditable` _papertilemap)
  (`PaperTileMapComponent.AddNewLayer` _papertilemap_2)
  (bind (_mapwidth _mapheight) (`PaperTileMapComponent.GetMapSize` _papertilemap_2))
  (bind _returnvalue_2 (- (* _mapwidth _mapheight) 1))
  (set `self.LastIndex` _returnvalue_2)
  (for _index (range (+ _returnvalue_2 1))
    (`PaperTileMapComponent.SetTile` (`self.PaperTileMap`) (/ _index _mapwidth) (mod _index _mapwidth) 0 (`TileMapBlueprintLibrary.MakeTile` 0 (`|GetArrayItem` (`self.TileSets`) _returnvalue)))
    (`self.RandomBranch` _returnvalue)))

(event `InputAction|Click`
  (params (Key :type "Key Structure"))
  (bind _tiledata (make `/Game/TileData` null))
  (bind _papertilemap (`self.PaperTileMap`))
  (bind _x (`self.X`))
  (bind _y (`self.Y`))
  (bind _tileset (break `/Game/TileData` (`self.FirstTile`)))
  (bind (_tileset_2 _x_2 _y_2) (break `/Game/TileData` (`self.FirstTile`)))
  (bind (_tileset_3 _x_3 _y_3) (break `/Game/TileData` (`self.SecondTile`)))
  (:`Pressed`
    (bind _returnvalue (`WidgetLayoutLibrary.GetMousePositionOnViewport`))
    (bind _returnvalue_2 (`KismetMathLibrary.FTrunc` (/ (`KismetMathLibrary.BreakVector2D` _returnvalue) 128.0)))
    (set `self.X` _returnvalue_2)
    (bind _returnvalue_3 (`KismetMathLibrary.FTrunc` (/ (`.Y` (`KismetMathLibrary.BreakVector2D` _returnvalue)) 128.0)))
    (set `self.Y` _returnvalue_3)
    (`/Engine/EditorBlueprintResources/StandardMacros.IsValid` _tileset
      (:`Is Valid`
        (bind (_returnvalue_tileindex _returnvalue_tileset) (break `PaperTileInfo` (`PaperTileMapComponent.GetTile` (`self.PaperTileMap`) _returnvalue_2 _returnvalue_3 0)))
        (if (== _tileset _returnvalue_tileset)
          (set `self.FirstTile` (make `/Game/TileData` null))
          (`PaperTileMapComponent.SetTile` (`self.PaperTileMap`) (`self.BGX`) (`self.BGY`) 1 (make `PaperTileInfo` 0))
          (else
            (`/Engine/EditorBlueprintResources/StandardMacros.IsValid` (`.TileSet_3_A51C73054906116F760C71AF5162EE34` (break `/Game/TileData` (`self.SecondTile`)))
              (:`Is Not Valid`
                (set `self.SecondTile` (make `/Game/TileData` _returnvalue_tileset (`self.X`) (`self.Y`)))
                (`PaperTileMapComponent.SetTile` _papertilemap _x_2 _y_2 0 (make `PaperTileInfo` 0 _tileset_3))
                (`PaperTileMapComponent.SetTile` _papertilemap _x_3 _y_3 0 (make `PaperTileInfo` 0 _tileset_2))
                (set `self.FirstTile` _tiledata)
                (set `self.SecondTile` _tiledata)
                (`PaperTileMapComponent.SetTile` (`self.PaperTileMap`) (`self.BGX`) (`self.BGY`) 1 (make `PaperTileInfo` 0)))))))
      (:`Is Not Valid`
        (set `self.FirstTile` (make `/Game/TileData` _returnvalue_tileset _returnvalue_2 _returnvalue_3))
        (`PaperTileMapComponent.SetTile` (`self.PaperTileMap`) _x _y 1 (make `PaperTileInfo` 0 "/Game/Tile/BG_set.BG_set"))
        (set `self.BGX` _x)
        (set `self.BGY` _y)))))

(fn `RandomBranch`
  (params (RandomNum :type Integer))
  (if (== RandomNum 0)
    (bind _result (`/Engine/EditorBlueprintResources/StandardMacros.IncrementInt` (`self.BoomNum`))
      (:`  `
        (if (>= _result 4)
          (set `self.Min` 1))))
    (elif (== RandomNum 5)
      (bind _result_2 (`/Engine/EditorBlueprintResources/StandardMacros.IncrementInt` (`self.StoneNum`))
        (:`  `
          (if (>= _result_2 4)
            (set `self.Max` 4)))))))

(fn `UserConstructionScript`)