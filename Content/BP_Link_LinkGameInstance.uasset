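; Game instance for the Link game that holds level data and shows end-of-game screens.
; Init fills three integer arrays: Level1 and Level2 cover consecutive, non-overlapping ranges, and Level3 combines both.
; Succeed and GameOver events create the Succeed or Defeated widget, add it to the viewport and switch the first player controller to UI-only input.
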(event `self.ReceiveInit`
  (set `self.Level_1` (`|MakeArray` "/Game/Texture/1/1.1" "/Game/Texture/1/2.2" "/Game/Texture/1/3.3" "/Game/Texture/1/4.4" "/Game/Texture/1/5.5" "/Game/Texture/1/6.6" "/Game/Texture/1/7.7" "/Game/Texture/1/8.8" "/Game/Texture/1/9.9" "/Game/Texture/1/10.10" "/Game/Texture/1/11.11" "/Game/Texture/1/12.12" "/Game/Texture/1/13.13" "/Game/Texture/1/14.14" "/Game/Texture/1/15.15" "/Game/Texture/1/16.16" "/Game/Texture/1/17.17" "/Game/Texture/1/18.18" :!type "Texture2D Object Reference"))
  (set `self.Level_2` (`|MakeArray` "/Game/Texture/2/19.19" "/Game/Texture/2/20.20" "/Game/Texture/2/21.21" "/Game/Texture/2/22.22" "/Game/Texture/2/23.23" "/Game/Texture/2/24.24" "/Game/Texture/2/25.25" "/Game/Texture/2/26.26" "/Game/Texture/2/27.27" "/Game/Texture/2/28.28" "/Game/Texture/2/29.29" "/Game/Texture/2/30.30" "/Game/Texture/2/31.31" "/Game/Texture/2/32.32" "/Game/Texture/2/33.33" "/Game/Texture/2/34.34" "/Game/Texture/2/35.35" "/Game/Texture/2/36.36" "/Game/Texture/2/37.37" "/Game/Texture/2/38.38" "/Game/Texture/2/39.39" "/Game/Texture/2/40.40" "/Game/Texture/2/41.41" "/Game/Texture/2/42.42" "/Game/Texture/2/43.43" "/Game/Texture/2/44.44" "/Game/Texture/2/45.45" "/Game/Texture/2/46.46" "/Game/Texture/2/47.47" "/Game/Texture/2/48.48" "/Game/Texture/2/49.49" "/Game/Texture/2/50.50" :!type "Texture2D Object Reference"))
  (set `self.Level_3` (`self.Level_1`))
  (`KismetArrayLibrary.Array_Append` (`self.Level_3`) (`self.Level_2`)))

(event `self.Succeed`
  (bind _returnvalue (`GameplayStatics.GetPlayerController` 0))
  (bind _returnvalue_2 (`|CreateWidget` "/Game/UI/Succeed.Succeed_C" _returnvalue))
  (`UserWidget.AddToViewport` _returnvalue_2 0)
  (`WidgetBlueprintLibrary.SetInputMode_UIOnlyEx` _returnvalue _returnvalue_2))

(event `self.GameOver`
  (bind _returnvalue (`GameplayStatics.GetPlayerController` 0))
  (bind _returnvalue_2 (`|CreateWidget` "/Game/UI/Defeated.Defeated_C" _returnvalue))
  (`UserWidget.AddToViewport` _returnvalue_2 0)
  (`WidgetBlueprintLibrary.SetInputMode_UIOnlyEx` _returnvalue _returnvalue_2))